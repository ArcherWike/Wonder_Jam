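; Flower enemy NPC that turns its mesh every tick to face the player on yaw only and reports itself as targettable.
; On BeginPlay it tints and sets its health bar widget and plays a camera shutter sound.
; The Kill event shows a dying line in the existing Text_WB and removes it, then spawns death effects, stops tick and movement, ragdolls the mesh and destroys the actor after a delay.
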(event EventTick
  (params (DeltaSeconds :type Float%20%28single-precision%29))
  (bind _mesh (Variables|Character|GetMesh))
  ;[1 1 1] Set Aim rotation
  (Transformation|SetWorldRotation _mesh (Math|Rotator|MakeRotator 0.0 0.0 (+ (.Yaw (Math|Rotator|BreakRotator (Math|Rotator|FindLookatRotation (Transformation|GetWorldLocation _mesh) (Transformation|GetActorLocation (Game|GetPlayerCharacter 0))))) -1e+02)) false false))

(event EventBeginPlay
  (bind _aswb_enemy_health_bar (Utilities|Casting|CastToWB_EnemyHealthBar (UserInterface|GetUserWidgetObject (Variables|Default|GetHealthBar))))
  (Class|ProgressBar|SetFillColorandOpacity (Variables|/Game/UI/Healthbars/WB_EnemyHealthBar.WB_EnemyHealthBar_C|GetProgressBar _aswb_enemy_health_bar) "(R=0.898021,G=0.000000,B=1.000000,A=1.000000)")
  (Variables|/Game/UI/Healthbars/WB_EnemyHealthBar.WB_EnemyHealthBar_C|SetHP%25 _aswb_enemy_health_bar 0.25)
  (Audio|PlaySoundatLocation "/Engine/VREditor/Sounds/UI/Camera_Shutter.Camera_Shutter" (Transformation|GetActorLocation) "0, 0, 0" 1.0 1.0 0.0 0 0 0 0))

(event EventKill
  ;[1 1 1] Kill npc
  (bind _foundwidgets (Widget|GetAllWidgetsOfClass "/Game/UI/Text_WB.Text_WB_C" true))
  (bind _output_get (Variables|Default|SetAs%20WB%20Text (Utilities|Array|Get(acopy) _foundwidgets)))
  (Variables|/Game/UI/Text_WB.Text_WB_C|SetText _output_get "Enemy: Noooooo!")
  (Utilities|FlowControl|Delay 1.0)
  (Widget|RemovefromParent (Variables|Default|GetAs%20WB%20Text))
  (Niagara|SpawnSystematLocation "/Game/Art/VFX/Flowers/N_FlowerDeath.N_FlowerDeath" (Transformation|GetActorLocation))
  (Audio|PlaySoundatLocation 0 "0, 0, 0" "0, 0, 0" 1.0 1.0 0.0 0 0 0 0)
  (Actor|Tick|SetActorTickEnabled false)
  (Physics|SetSimulatePhysics (Variables|Character|GetMesh) true)
  (Pawn|Components|CharacterMovement|DisableMovement (Variables|Character|GetCharacterMovement))
  (Utilities|FlowControl|Delay 3.0)
  (Actor|DestroyActor))

(fn ConstructionScript)

(fn IsTargettable
  (return true))