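; BP_Flower is a ranged AI opponent that feeds its blackboard with targets and can be killed once weakened.
; Each tick it picks the closest valid actor inside its attack-range sphere, while pawn sensing flags player sightings.
; Damage updates health through the game mode's DamageManager, setting Killable at a health threshold.
; Kill then triggers death and, if targeted, clears the player's targeter and notifies the hero, using data-table stats and effects.
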(event OnSeePawn(PawnSensing)
  (params (Pawn :type Pawn%20Object%20Reference))
  (bind _self self)
  (bind _returnvalue (AI|GetAIController _self))
  (bind _returnvalue_2 (AI|GetBlackboard _returnvalue))
  ;[1 1 1] Check if player seen
  (if (Pawn|IsPlayerControlled Pawn)
    (AI|Components|Blackboard|SetValueasBool _returnvalue_2 (Utilities|Name|MakeLiteralName "PlayerSeen") true)
    (else
      (AI|Components|Blackboard|SetValueasBool _returnvalue_2 (Utilities|Name|MakeLiteralName "PlayerSeen") false))))

(event Game|Damage|EventAnyDamage
  (params (Damage :type Float%20%28single-precision%29) (DamageType :type Damage%20Type%20Object%20Reference) (InstigatedBy :type Controller%20Object%20Reference) (DamageCauser :type Actor%20Object%20Reference))
  (bind _damage_manager (Variables|Default|GetDamage%20Manager))
  ;[1 1 1] Take data from data base
  (bind _returnvalue (Utilities|GetDataTableRow "/Game/Systems/DT_Character.DT_Character" (Variables|Default|GetName))
    (:then
      ;[1 1 1] Change HP
      (bind (_hp_ _newhealth) (Default|UpdateHealthBar (Variables|Default|GetDamage%20Manager) (Variables|Default|GetHealth) Damage (.HP (Utilities|Struct|BreakCharacterStats _returnvalue)) (Variables|Default|GetHealthBar)))
      (Variables|Default|SetHealth _newhealth)
      ;[1 1 1] Check if deadable
      (if (== _hp_ 0.25)
        (Default|SetHealthbarLook _damage_manager (Variables|Default|GetHealthBar))
        (Variables|Default|SetKillable true)
        (else
          (Default|Hurt _damage_manager (.HurtSound (Utilities|Struct|BreakCharacterStats _returnvalue)) (.HurtEffect (Utilities|Struct|BreakCharacterStats _returnvalue)) self))))))

(event EventTick
  (params (DeltaSeconds :type Float%20%28single-precision%29))
  ;[1 1 1] Set Target
  (CallFunction|SetClosestTarget))

(event EventBeginPlay
  (bind _name (Variables|Default|GetName))
  ;[1 1 1] Set enemy counter
  (bind _ashero (Utilities|Casting|CastToHero (Game|GetPlayerCharacter 0)))
  (Default|EnemyCounter _ashero)
  ;[1 1 1] Set game manager
  (bind _ashero_game_mode (Utilities|Casting|CastToHeroGameMode (Game|GetGameMode)))
  (Variables|Default|SetDamage%20Manager (Variables|/Game/GameMods/HeroGameMode.HeroGameMode_C|GetDamage%20Manager _ashero_game_mode))
  ;[1 1 1] Set HP
  (bind _returnvalue (Utilities|GetDataTableRow "/Game/Systems/DT_Character.DT_Character" (Variables|Default|GetName))
    (:then
      (bind _output_get (Variables|Default|SetHealth (.HP (Utilities|Struct|BreakCharacterStats _returnvalue))))
      (Default|SetHealthBar (Variables|Default|GetDamage%20Manager) _output_get (Variables|Default|GetHealthBar))
      ;[1 1 1] set name
      (Class|BlackboardComponent|SetValueasName (Variables|/Script/AIModule.AIController|GetBlackboard (AI|GetAIController self)) (Utilities|Name|MakeLiteralName "Name") _name)
      ;[1 1 1] set sphere radius (TargetNet)
      (bind _returnvalue_2 (Utilities|GetDataTableRow "/Game/Systems/DT_Attack.DT_Attack" _name)
        (:then
          (Components|Sphere|SetSphereRadius (Variables|Default|GetTargetNet) (Math|Conversions|ToFloat(Integer) (.AttackRange (Utilities|Struct|BreakAttackStats _returnvalue_2))) true))))))

(event EventKill
  ;[1 1 1] If killable, kill
  (if (Variables|Default|GetKillable)
    (Default|Death (Variables|Default|GetDamage%20Manager) (.DeathSound (Utilities|Struct|BreakCharacterStats (stale Game|Damage|EventAnyDamage _returnvalue))) (.DeathEffect (Utilities|Struct|BreakCharacterStats (stale Game|Damage|EventAnyDamage _returnvalue))) self)
    ;[1 1 1] if it's target kill this object
    (bind _ashero_player_controller (Utilities|Casting|CastToHeroPlayerController (Game|GetPlayerController 0)))
    (if (== (Variables|/Game/GameMods/HeroPlayerController.HeroPlayerController_C|GetCurrentTarget _ashero_player_controller) self)
      (Actor|DestroyActor (Variables|/Game/GameMods/HeroPlayerController.HeroPlayerController_C|GetTargetterActorRef _ashero_player_controller))
      (bind _ashero (Utilities|Casting|CastToHero (Game|GetPlayerCharacter 0)))
      (Default|EnemyDeath _ashero))))

(fn ConstructionScript)

(fn SetClosestTarget
  (bind _self self)
  (bind _self_2 self)
  (bind _returnvalue (AI|GetBlackboard _self))
  (bind _returnvalue_2 (AI|GetBlackboard _self_2))
  ;[1 1 1] start with larger value of closest distance than you can have
  (Variables|Default|SetClosestDistance (+ (Variables|/Script/Engine.SphereComponent|GetSphereRadius (Variables|Default|GetTargetNet)) 1e+01))
  ;[1 1 1] add overlapping actors to Array (Target in Range)
  (for _array_element (Collision|GetOverlappingActors (Variables|Default|GetTargetNet) 0 :!class /Script/Engine.PrimitiveComponent)
    (bind _is_opponent (Class|IsFlowerOpponent|IsFlowerOpponent(Message) _array_element))
    (if _is_opponent
      (Utilities|Array|AddUnique (LocalVariables|GetTargetInRangeArray) _array_element)
      ;[1 1 1] check and change the closest distance
      (if (< (Transformation|GetDistanceTo _array_element self) (Variables|Default|GetClosestDistance))
        (Variables|Default|SetClosestDistance (Transformation|GetDistanceTo _array_element self))
        (Variables|Default|SetClosestTarget _array_element))))
  (if (> (Utilities|Array|Length (LocalVariables|GetTargetInRangeArray)) 0)
    ;[1 1 1] Set in range, target in AI blackboard
    (AI|Components|Blackboard|SetValueasBool _returnvalue (Utilities|Name|MakeLiteralName "TargetInRange") true)
    (AI|Components|Blackboard|SetValueasObject _returnvalue (Utilities|Name|MakeLiteralName "Target") (Variables|Default|GetClosestTarget))
    (else
      ;[1 1 1] can't see target - set AI Blackboard
      (AI|Components|Blackboard|SetValueasBool _returnvalue_2 (Utilities|Name|MakeLiteralName "TargetInRange") false)
      (bind _output_get (Variables|Default|SetClosestTarget (Variables|Default|GetNone_Obj)))
      (AI|Components|Blackboard|SetValueasObject _returnvalue_2 (Utilities|Name|MakeLiteralName "Target") _output_get))))

(fn CanAttackFlower
  (if (Variables|Default|GetKillable)
    (return false)
    (else
      (return true))))

(fn IsTargettable
  (return true))